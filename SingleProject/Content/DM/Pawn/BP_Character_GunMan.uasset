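; Gunman character Blueprint that fires a hitscan laser on left mouse click.
; A long Visibility line trace runs from the camera manager's location along its forward vector, drawing a brief debug line.
; On a hit, it spawns BP_MasterField at the impact point and calls ApplyDamage, though no damaged actor is wired to that call.
; A node to destroy the hit actor is present but disconnected.
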(event `Key|LeftMouseButton`
  (params (Key :type "Key Structure"))
  (bind _returnvalue (`GameplayStatics.GetPlayerCameraManager` 0))
  (bind _returnvalue_2 (`self.K2_GetActorLocation` _returnvalue))
  ;[1 1 1] 레이저
  (:`Pressed`
    (bind (_outhit _returnvalue_3) (`KismetSystemLibrary.LineTraceSingle` :`Start` _returnvalue_2 :`End` (+ _returnvalue_2 (* (`KismetMathLibrary.GetForwardVector` (`self.K2_GetActorRotation` _returnvalue)) 100000.0)) :`TraceChannel` "TraceTypeQuery1" :`DrawDebugType` "ForDuration" :`DrawTime` 0.5))
    (if _returnvalue_3
      (`GameplayStatics.ApplyDamage` null 1.0)
      (`|SpawnActorFromClass` "/Game/DM/Fracture/BP_MasterField.BP_MasterField_C" (`KismetMathLibrary.Conv_VectorToTransform` (`.Location` (`GameplayStatics.BreakHitResult` _outhit))) "Undefined" "MultiplyWithRoot" null null))))

(fn `UserConstructionScript`)