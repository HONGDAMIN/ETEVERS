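; BP_Block_Y is a moving obstacle block that oscillates along its local Y axis and knocks the player character on contact.
; Tick applies a frame-rate-dependent step scaled by XMultiplyY, flipping MoveY when the accumulated offset passes either limit.
; Sphere hits on BP_ThirdPersonCharacter add a velocity-change impulse to its movement component.
; The impulse look-at uses the character's location as both start and target, so it always points along world X.
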(event `self.Sphere.OnComponentHit`
  (params (HitComponent :type "PrimitiveComponent Object Reference") (OtherActor :type "Actor Object Reference") (OtherComp :type "PrimitiveComponent Object Reference") (NormalImpulse :type "Vector Structure") (Hit :type "HitResult Structure (by ref)"))
  ;[1 1 1] 충돌 충격
  (bind _asbp_third_person_character (cast `/Game/ThirdPerson/Blueprints/BP_ThirdPersonCharacter` (`.HitActor` (`GameplayStatics.BreakHitResult` Hit))))
  (bind (_returnvalue_x _returnvalue_y _returnvalue_z) (`KismetMathLibrary.BreakVector` (* (`KismetMathLibrary.GetForwardVector` (`KismetMathLibrary.FindLookAtRotation` (`self.K2_GetActorLocation` _asbp_third_person_character) (`self.K2_GetActorLocation` _asbp_third_person_character))) 5000.0)))
  (`CharacterMovementComponent.AddImpulse` (`Character.CharacterMovement` _asbp_third_person_character) (`KismetMathLibrary.MakeVector` _returnvalue_x _returnvalue_y _returnvalue_z) true))

(event `self.ReceiveTick`
  (params (DeltaSeconds :type "Float (single-precision)"))
  (bind _returnvalue (* (`self.XMultiply_Y`) 10.0))
  (bind _returnvalue_2 (* (`self.XMultiply_Y`) -10.0))
  ;[1 1 1] 액터 이동
  (if (`self.Move_Y`)
    (`self.K2_AddActorLocalOffset` (`KismetMathLibrary.MakeVector` 0.0 _returnvalue))
    (set `self.LocalOffset_Y` (+ (`self.LocalOffset_Y`) _returnvalue))
    (if (> (`self.LocalOffset_Y`) 300.0)
      (set `self.Move_Y` false))
    (else
      (`self.K2_AddActorLocalOffset` (`KismetMathLibrary.MakeVector` 0.0 _returnvalue_2))
      (set `self.LocalOffset_Y` (+ (`self.LocalOffset_Y`) _returnvalue_2))
      (if (< (`self.LocalOffset_Y`) -300.0)
        (set `self.Move_Y` true)))))

(fn `UserConstructionScript`)