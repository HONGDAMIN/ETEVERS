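; BP_Final_Block is a moving obstacle actor that knocks the third-person character on contact.
; Each Tick it shifts equally on all local axes, scaled by FinalMultiply, reversing via FinalMove when the tracked offset passes ±200, independent of delta time.
; A Sphere hit applies a velocity-change impulse to the character.
; Its look-at uses the character's location as both start and target, so the push ignores the block's position.
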(event `self.ReceiveTick`
  (params (DeltaSeconds :type "Float (single-precision)"))
  (bind _final_multiply (`self.Final_Multiply`))
  (bind _final_localoffset (`self.Final_LocalOffset`))
  (bind _final_localoffset_2 (`self.Final_LocalOffset`))
  (bind _returnvalue (* _final_multiply 10.0))
  (bind _returnvalue_2 (* _final_multiply -10.0))
  ;[1 1 1] 액터 이동
  (if (`self.Final_Move`)
    (`self.K2_AddActorLocalOffset` (`KismetMathLibrary.MakeVector` _returnvalue _returnvalue _returnvalue))
    (set `self.Final_LocalOffset` (+ _final_localoffset _returnvalue))
    (if (> _final_localoffset_2 200.0)
      (set `self.Final_Move` false))
    (else
      (`self.K2_AddActorLocalOffset` (`KismetMathLibrary.MakeVector` _returnvalue_2 _returnvalue_2 _returnvalue_2))
      (set `self.Final_LocalOffset` (+ _final_localoffset _returnvalue_2))
      (if (< _final_localoffset_2 -200.0)
        (set `self.Final_Move` true)))))

(event `self.Sphere.OnComponentHit`
  (params (HitComponent :type "PrimitiveComponent Object Reference") (OtherActor :type "Actor Object Reference") (OtherComp :type "PrimitiveComponent Object Reference") (NormalImpulse :type "Vector Structure") (Hit :type "HitResult Structure (by ref)"))
  ;[1 1 1] 충돌 충격
  (bind _asbp_third_person_character (cast `/Game/ThirdPerson/Blueprints/BP_ThirdPersonCharacter` (`.HitActor` (`GameplayStatics.BreakHitResult` Hit))))
  (bind (_returnvalue_x _returnvalue_y _returnvalue_z) (`KismetMathLibrary.BreakVector` (* (`KismetMathLibrary.GetForwardVector` (`KismetMathLibrary.FindLookAtRotation` (`self.K2_GetActorLocation` _asbp_third_person_character) (`self.K2_GetActorLocation` _asbp_third_person_character))) 2000.0)))
  (`CharacterMovementComponent.AddImpulse` (`Character.CharacterMovement` _asbp_third_person_character) (`KismetMathLibrary.MakeVector` _returnvalue_x _returnvalue_y _returnvalue_z) true))

(fn `UserConstructionScript`)