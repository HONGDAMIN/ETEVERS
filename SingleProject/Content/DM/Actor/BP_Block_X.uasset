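; BP_Block_X is a moving obstacle that shuttles along its local X axis and knocks back the third-person character on contact.
; Tick offsets the actor by a per-frame step scaled by XMultiply, flipping Move when the tracked offset passes either limit, without delta-time scaling.
; Sphere hits add a velocity-change impulse to the character's movement, with look-at start and target both the character's location, so direction ignores the block.
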(event `self.Sphere.OnComponentHit`
  (params (HitComponent :type "PrimitiveComponent Object Reference") (OtherActor :type "Actor Object Reference") (OtherComp :type "PrimitiveComponent Object Reference") (NormalImpulse :type "Vector Structure") (Hit :type "HitResult Structure (by ref)"))
  ;[1 1 1] 충돌 충격
  (bind _asbp_third_person_character (cast `/Game/ThirdPerson/Blueprints/BP_ThirdPersonCharacter` (`.HitActor` (`GameplayStatics.BreakHitResult` Hit))))
  (bind (_returnvalue_x _returnvalue_y _returnvalue_z) (`KismetMathLibrary.BreakVector` (* (`KismetMathLibrary.GetForwardVector` (`KismetMathLibrary.FindLookAtRotation` (`self.K2_GetActorLocation` _asbp_third_person_character) (`self.K2_GetActorLocation` _asbp_third_person_character))) 5000.0)))
  (`CharacterMovementComponent.AddImpulse` (`Character.CharacterMovement` _asbp_third_person_character) (`KismetMathLibrary.MakeVector` _returnvalue_x _returnvalue_y _returnvalue_z) true))

(event `self.ReceiveTick`
  (params (DeltaSeconds :type "Float (single-precision)"))
  (bind _returnvalue (* (`self.X_Multiply`) 5.0))
  (bind _returnvalue_2 (* (`self.X_Multiply`) -5.0))
  ;[1 1 1] 물체 이동
  (if (`self.Move`)
    (`self.K2_AddActorLocalOffset` (`KismetMathLibrary.MakeVector` _returnvalue))
    (set `self.Localoffset` (+ (`self.Localoffset`) _returnvalue))
    (if (> (`self.Localoffset`) 300.0)
      (set `self.Move` false))
    (else
      (`self.K2_AddActorLocalOffset` (`KismetMathLibrary.MakeVector` _returnvalue_2))
      (set `self.Localoffset` (+ (`self.Localoffset`) _returnvalue_2))
      (if (< (`self.Localoffset`) -300.0)
        (set `self.Move` true)))))

(fn `UserConstructionScript`)