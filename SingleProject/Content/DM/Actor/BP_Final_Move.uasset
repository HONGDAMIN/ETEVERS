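; BP_Final_Move is an actor that travels along a fixed three-leg path once BP_ThirdPersonCharacter overlaps its Box.
; The overlap starts a 0.01-second looping timer, which nudges the actor by local offsets scaled by Multiply.
; While Condtion holds it moves along +Y, then down Z, then along +X, tracking accumulated distance against hardcoded limits.
; The timer is never cleared, even after the final limit is reached.
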(event `self.ReceiveTick`
  (params (DeltaSeconds :type "Float (single-precision)")))

(event `self.Box.OnComponentBeginOverlap`
  (params (OverlappedComponent :type "PrimitiveComponent Object Reference") (OtherActor :type "Actor Object Reference") (OtherComp :type "PrimitiveComponent Object Reference") (OtherBodyIndex :type Integer) (bFromSweep :type Boolean) (SweepResult :type "HitResult Structure (by ref)"))
  ;[1 1 1] 오버랩시 지정된 위치로 이동
  (cast `/Game/ThirdPerson/Blueprints/BP_ThirdPersonCharacter` OtherActor)
  (`KismetSystemLibrary.K2_SetTimerDelegate` (delegate `CustomEvent`) 0.01 true))

(event `CustomEvent`
  (bind _returnvalue (* (`self.Multiply`) 100.0))
  (bind _returnvalue_2 (* (`self.Multiply`) 100.0))
  (bind _returnvalue_3 (* (`self.Multiply`) -100.0))
  ;[1 1 1] 오버랩시 지정된 위치로 이동
  (if (`self.condtion`)
    (`self.K2_AddActorLocalOffset` (`KismetMathLibrary.MakeVector` 0.0 _returnvalue))
    (set `self.MoveLocaloffsetY` (+ (`self.MoveLocaloffsetY`) _returnvalue))
    (if (> (`self.MoveLocaloffsetY`) 29180.0)
      (set `self.condtion` false))
    (elif (> (`self.MoveLocaloffsetZ`) -10680.0)
      (`self.K2_AddActorLocalOffset` (`KismetMathLibrary.MakeVector` 0.0 0.0 _returnvalue_3))
      (set `self.MoveLocaloffsetZ` (+ (`self.MoveLocaloffsetZ`) _returnvalue_3))
      (elif (< (`self.MoveLocaloffsetX`) 2460.0)
        (`self.K2_AddActorLocalOffset` (`KismetMathLibrary.MakeVector` _returnvalue_2))
        (set `self.MoveLocaloffsetX` (+ (`self.MoveLocaloffsetX`) _returnvalue_2))))))

(fn `UserConstructionScript`)