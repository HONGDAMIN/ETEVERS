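; BP_Stage2Move is an actor that moves from its starting location toward a target actor once the player character type enters its box.
; It stores its location at BeginPlay, and an overlap by BP_ThirdPersonCharacter plays a timeline.
; Each timeline update lerps between the stored location and the valid TargetActor's current location, setting the position without sweep.
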(event `self.ReceiveBeginPlay`
  (set `self.InitLcation` (`self.K2_GetActorLocation`)))

(event `self.Box.OnComponentBeginOverlap`
  (params (OverlappedComponent :type "PrimitiveComponent Object Reference") (OtherActor :type "Actor Object Reference") (OtherComp :type "PrimitiveComponent Object Reference") (OtherBodyIndex :type Integer) (bFromSweep :type Boolean) (SweepResult :type "HitResult Structure (by ref)"))
  (bind _targetactor (`self.TargetActor`))
  (cast `/Game/ThirdPerson/Blueprints/BP_ThirdPersonCharacter` OtherActor)
  (bind (_direction _newtrack_0) (`Timeline|Timeline`)
    (:`Update`
      (`/Engine/EditorBlueprintResources/StandardMacros.IsValid` _targetactor
        (:`Is Valid`
          (`self.K2_SetActorLocation` (`KismetMathLibrary.VLerp` (`self.InitLcation`) (`self.K2_GetActorLocation` _targetactor) _newtrack_0)))))))

(fn `UserConstructionScript`)