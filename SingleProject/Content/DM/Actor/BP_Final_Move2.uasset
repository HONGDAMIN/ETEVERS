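; BP_Final_Move2 is an actor that slides along its local negative X axis once the third-person character overlaps its Box.
; The overlap starts a fast looping timer that offsets the actor by a step scaled by Multuply and accumulates the distance in LocaloffsetX.
; The -2000 limit check leads to no action, so nothing in the Blueprint stops the movement.
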(event `self.Box.OnComponentBeginOverlap`
  (params (OverlappedComponent :type "PrimitiveComponent Object Reference") (OtherActor :type "Actor Object Reference") (OtherComp :type "PrimitiveComponent Object Reference") (OtherBodyIndex :type Integer) (bFromSweep :type Boolean) (SweepResult :type "HitResult Structure (by ref)"))
  ;[1 1 1] 오버랩시 x축 이동
  (cast `/Game/ThirdPerson/Blueprints/BP_ThirdPersonCharacter` OtherActor)
  (`KismetSystemLibrary.K2_SetTimerDelegate` (delegate `CustomEvent`) 0.01 true))

(event `CustomEvent`
  (bind _returnvalue (* (`self.multuply`) -10.0))
  ;[1 1 1] 오버랩시 x축 이동
  (`self.K2_AddActorLocalOffset` (`KismetMathLibrary.MakeVector` _returnvalue))
  (set `self.localoffsetX` (+ (`self.localoffsetX`) _returnvalue))
  (if (> (`self.localoffsetX`) -2000.0)
    _))

(fn `UserConstructionScript`)