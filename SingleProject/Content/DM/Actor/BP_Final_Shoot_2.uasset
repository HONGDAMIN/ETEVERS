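; BP_Final_Shoot_2 is an actor with a Sphere that knocks the player character away when it registers a hit.
; BeginPlay turns off physics simulation on the Sphere and clears the Physics flag.
; On hit, it casts to BP_ThirdPersonCharacter and applies a strong velocity-change impulse through CharacterMovement.
; The look-at rotation uses the character's location as both start and target, so the push direction ignores the sphere's position.
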(event `self.Sphere.OnComponentHit`
  (params (HitComponent :type "PrimitiveComponent Object Reference") (OtherActor :type "Actor Object Reference") (OtherComp :type "PrimitiveComponent Object Reference") (NormalImpulse :type "Vector Structure") (Hit :type "HitResult Structure (by ref)"))
  ;[1 1 1] 부딪
  (bind _asbp_third_person_character (cast `/Game/ThirdPerson/Blueprints/BP_ThirdPersonCharacter` (`.HitActor` (`GameplayStatics.BreakHitResult` Hit))))
  (bind (_returnvalue_x _returnvalue_y _returnvalue_z) (`KismetMathLibrary.BreakVector` (* (`KismetMathLibrary.GetForwardVector` (`KismetMathLibrary.FindLookAtRotation` (`self.K2_GetActorLocation` _asbp_third_person_character) (`self.K2_GetActorLocation` _asbp_third_person_character))) 8000.0)))
  (`CharacterMovementComponent.AddImpulse` (`Character.CharacterMovement` _asbp_third_person_character) (`KismetMathLibrary.MakeVector` _returnvalue_x _returnvalue_y _returnvalue_z) true))

(event `self.ReceiveBeginPlay`
  ;[1 1 1] 시뮬레이트 끄기
  (`PrimitiveComponent.SetSimulatePhysics` (`self.Sphere`) false)
  (set `self.Physics` false))

(fn `UserConstructionScript`)